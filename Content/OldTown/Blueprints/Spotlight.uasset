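; Configurable spotlight fixture actor for the OldTown content, set up entirely in the construction script with no active gameplay logic.
; Normalized Rotation and Swivle values turn the Pivot in yaw and the Light component in pitch over a full circle.
; LightOnOff set to true switches the fixture off, zeroing both the dynamic material's emissive strength and the SpotLight intensity; false makes it glow at LightIntensity.
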(event EventBeginPlay)

(event Collision|EventActorBeginOverlap
  (params (OtherActor :type Actor%20Object%20Reference)))

(event EventTick
  (params (DeltaSeconds :type Float%20%28single-precision%29)))

(fn ConstructionScript
  (bind _spotlight (Variables|Default|GetSpotLight))
  (bind _returnvalue (Rendering|Material|CreateDynamicMaterialInstance (Variables|Default|GetLight) 0 "/Game/OldTown/Materials/Spotlight.Spotlight" "None" :!class /Script/Engine.PrimitiveComponent))
  (Variables|Default|SetDMI _returnvalue)
  (Transformation|SetRelativeRotation (Variables|Default|GetLight) (Math|Rotator|MakeRotator 0.0 (* (Variables|Default|GetSwivle) 3.6e+02) 0.0) false false)
  (Transformation|SetRelativeRotation (Variables|Default|GetPivot) (Math|Rotator|MakeRotator 0.0 0.0 (* (Variables|Default|GetRotation) 3.6e+02)) false false)
  (if (Variables|Default|GetLight%20on/Off)
    (Rendering|Material|SetScalarParameterValue (Variables|Default|GetDMI) "Emissive Strength" 0.0 :!class /Script/Engine.MaterialInstanceDynamic)
    (Rendering|Components|Light|SetIntensity _spotlight 0.0)
    (else
      (Rendering|Material|SetScalarParameterValue (Variables|Default|GetDMI) "Emissive Strength" 1e+01 :!class /Script/Engine.MaterialInstanceDynamic)
      (Rendering|Components|Light|SetIntensity _spotlight (Variables|Default|GetLight%20Intensity)))))