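; Traffic light actor for the Old Town level that cycles two opposing signal faces through green, yellow and red.
; The construction script creates dynamic material instances on two material slots of the static mesh, one for each face.
; From BeginPlay, an endless Delay loop drives the Red, Yellow and Green scalar parameters on both instances, so one face shows red while the other runs green then yellow.
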(event EventBeginPlay
  (bind _lights (Variables|Default|GetLIghts))
  (bind _lights_2 (Variables|Default|GetLIghts))
  (bind _lights_alt (Variables|Default|GetLights%20Alt))
  (bind _lights_3 (Variables|Default|GetLIghts))
  (bind _lights_alt_2 (Variables|Default|GetLights%20Alt))
  (bind _lights_alt_3 (Variables|Default|GetLights%20Alt))
  (Rendering|Material|SetScalarParameterValue _lights_2 "Red" 25.0 :!class /Script/Engine.MaterialInstanceDynamic :!label _label)
  (Rendering|Material|SetScalarParameterValue _lights_2 "Green" 0.0 :!class /Script/Engine.MaterialInstanceDynamic)
  (Rendering|Material|SetScalarParameterValue _lights_2 "Yellow" 0.0 :!class /Script/Engine.MaterialInstanceDynamic)
  (Rendering|Material|SetScalarParameterValue _lights_alt "Red" 0.0 :!class /Script/Engine.MaterialInstanceDynamic)
  (Rendering|Material|SetScalarParameterValue _lights_alt "Green" 25.0 :!class /Script/Engine.MaterialInstanceDynamic)
  (Rendering|Material|SetScalarParameterValue _lights_alt "Yellow" 0.0 :!class /Script/Engine.MaterialInstanceDynamic)
  (Utilities|FlowControl|Delay 15.0)
  (Rendering|Material|SetScalarParameterValue _lights_alt_2 "Green" 0.0 :!class /Script/Engine.MaterialInstanceDynamic)
  (Rendering|Material|SetScalarParameterValue _lights_alt_2 "Yellow" 25.0 :!class /Script/Engine.MaterialInstanceDynamic)
  (Utilities|FlowControl|Delay 4.0)
  (Rendering|Material|SetScalarParameterValue _lights_3 "Red" 0.0 :!class /Script/Engine.MaterialInstanceDynamic)
  (Rendering|Material|SetScalarParameterValue _lights_3 "Green" 25.0 :!class /Script/Engine.MaterialInstanceDynamic)
  (Rendering|Material|SetScalarParameterValue _lights_3 "Yellow" 0.0 :!class /Script/Engine.MaterialInstanceDynamic)
  (Rendering|Material|SetScalarParameterValue _lights_alt_3 "Red" 25.0 :!class /Script/Engine.MaterialInstanceDynamic)
  (Rendering|Material|SetScalarParameterValue _lights_alt_3 "Green" 0.0 :!class /Script/Engine.MaterialInstanceDynamic)
  (Rendering|Material|SetScalarParameterValue _lights_alt_3 "Yellow" 0.0 :!class /Script/Engine.MaterialInstanceDynamic)
  (Utilities|FlowControl|Delay 15.0)
  (Rendering|Material|SetScalarParameterValue _lights "Green" 0.0 :!class /Script/Engine.MaterialInstanceDynamic)
  (Rendering|Material|SetScalarParameterValue _lights "Yellow" 25.0 :!class /Script/Engine.MaterialInstanceDynamic)
  (Utilities|FlowControl|Delay 4.0)
  (goto _label))

(event Collision|EventActorBeginOverlap
  (params (OtherActor :type Actor%20Object%20Reference)))

(event EventTick
  (params (DeltaSeconds :type Float%20%28single-precision%29)))

(fn ConstructionScript
  (bind _returnvalue (Rendering|Material|CreateDynamicMaterialInstance (Variables|Default|GetStaticMesh) 0 "/Game/OldTown/Materials/TrafficLight.TrafficLight" "None" :!class /Script/Engine.PrimitiveComponent))
  (Variables|Default|SetLIghts _returnvalue)
  (bind _returnvalue_2 (Rendering|Material|CreateDynamicMaterialInstance (Variables|Default|GetStaticMesh) 1 "/Game/OldTown/Materials/TrafficLight_Alt.TrafficLight_Alt" "None" :!class /Script/Engine.PrimitiveComponent))
  (Variables|Default|SetLights%20Alt _returnvalue_2))