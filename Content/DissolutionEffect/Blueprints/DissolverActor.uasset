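; DissolverActor is a dissolution effect volume that slices static meshes entering its box and drives a Niagara particle system.
; Each tick, it spawns a procedural-mesh Clone for every overlapping StaticMeshActor, then slices overlapping Clones at SCColor's position and forward vector.
; OrthoWidth sizes the capture component, plane and particle area.
; Construction and BeginPlay push size, lifetime, force and noise settings into Niagara.
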(event EventBeginPlay
  (bind _niagara (Variables|Default|GetNiagara))
  (Utilities|FlowControl|Sequence
    (:then_0
      (Niagara|SetNiagaraVariable(Float) _niagara "Size" (/ (Variables|Default|GetOrthoWidth) 2.0)))
    (:then_1
      (Niagara|SetNiagaraVariable(Float) _niagara "LifeTime" (Variables|Default|GetLifeTime)))
    (:then_2
      (Niagara|SetNiagaraVariable(Float) _niagara "Force" (Variables|Default|GetForce)))
    (:then_3
      (Niagara|SetNiagaraVariable(Float) _niagara "MaxDistance" (Variables|Default|GetMaxDistance)))
    (:then_4
      (Niagara|SetNiagaraVariable(Float) _niagara "NoiseStrength" (Variables|Default|GetNoiseStrength)))
    (:then_5
      (Niagara|SetNiagaraVariable(Float) _niagara "NoiseFrequency" (Variables|Default|GetNoiseFrequency)))
    (:then_6
      (Niagara|SetNiagaraVariable(Float) _niagara "ParticleSize" (Variables|Default|GetParticleSize)))))

(event EventTick
  (params (DeltaSeconds :type Float%20%28single-precision%29))
  (bind _box (Variables|Default|GetBox))
  (bind _box_2 (Variables|Default|GetBox))
  (bind _ignoreactororobject3 (Variables|Default|GetIgnoreActorOrObject3))
  (bind _ignoreactororobject1 (Variables|Default|GetIgnoreActorOrObject1))
  (bind _ignoreactororobject4 (Variables|Default|GetIgnoreActorOrObject4))
  (bind _sc_color (Variables|Default|GetSC_Color))
  (bind _ignoreactororobject2 (Variables|Default|GetIgnoreActorOrObject2))
  (bind _array (Utilities|Array|MakeArray _ignoreactororobject1 _ignoreactororobject2 _ignoreactororobject3 _ignoreactororobject4))
  (Utilities|FlowControl|Sequence
    (:then_0
      (bind (_outactors _returnvalue) (Collision|ComponentOverlapActors _box_2 (Transformation|GetWorldTransform _box_2) (Utilities|Array|MakeArray "ObjectTypeQuery1" "ObjectTypeQuery2" "ObjectTypeQuery4") "/Script/Engine.StaticMeshActor" _array))
      (if _returnvalue
        (for _array_element _outactors
          (bind _returnvalue_2 (Game|SpawnActorfromClass "/Game/DissolutionEffect/Blueprints/Clone.Clone_C" (Transformation|GetActorTransform _array_element) "AlwaysSpawn" 0 0))
          (Default|CreateProceduralMesh _returnvalue_2 _array_element))))
    (:then_1
      (bind (_outactors_2 _returnvalue_3) (Collision|ComponentOverlapActors _box (Transformation|GetWorldTransform _box) (Utilities|Array|MakeArray "ObjectTypeQuery1" "ObjectTypeQuery2" "ObjectTypeQuery4") "/Game/DissolutionEffect/Blueprints/Clone.Clone_C" _array))
      (if _returnvalue_3
        (for _array_element_2 _outactors_2
          (bind _asclone (Utilities|Casting|CastToClone _array_element_2))
          (Default|Slice _asclone (Transformation|GetWorldLocation _sc_color) (Math|Vector|GetForwardVector _sc_color)))))))

(fn ConstructionScript
  (bind _niagara (Variables|Default|GetNiagara))
  (Utilities|FlowControl|Sequence
    (:then_0
      (Variables|/Script/Engine.SceneCaptureComponent2D|SetOrthoWidth (Variables|Default|GetSC_Color) (Variables|Default|GetOrthoWidth)))
    (:then_1
      (Transformation|SetWorldScale3D (Variables|Default|GetPlane) (Math|Conversions|ToVector(Float) (/ (Variables|Default|GetOrthoWidth) 1e+02))))
    (:then_2
      (Utilities|FlowControl|Sequence
        (:then_0
          (Niagara|SetNiagaraVariable(Float) _niagara "Size" (/ (Variables|Default|GetOrthoWidth) 2.0)))
        (:then_1
          (Niagara|SetNiagaraVariable(Float) _niagara "LifeTime" (Variables|Default|GetLifeTime)))
        (:then_2
          (Niagara|SetNiagaraVariable(Float) _niagara "Force" (Variables|Default|GetForce)))
        (:then_3
          (Niagara|SetNiagaraVariable(Float) _niagara "MaxDistance" (Variables|Default|GetMaxDistance)))
        (:then_4
          (Niagara|SetNiagaraVariable(Float) _niagara "NoiseStrength" (Variables|Default|GetNoiseStrength)))
        (:then_5
          (Niagara|SetNiagaraVariable(Float) _niagara "NoiseFrequency" (Variables|Default|GetNoiseFrequency)))))))