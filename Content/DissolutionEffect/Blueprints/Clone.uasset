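; Clone actor that replaces a source actor with procedural mesh copies that can be sliced by a plane.
; CreateProceduralMesh copies each static mesh component into a procedural mesh at the same world transform, adds convex collision from section 0 vertices, then destroys the source.
; Slice cuts every procedural mesh on the actor at a given position and normal, without capping the cut.
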(event Custom|CreateProceduralMesh
  (params (ActorSource :type Actor%20Object%20Reference))
  (for _array_element (Actor|GetComponentsByClass ActorSource "/Script/Engine.StaticMeshComponent")
    (bind _returnvalue (AddComponent|AddProceduralMeshComponent true (Transformation|GetWorldTransform _array_element)))
    (Class|KismetProceduralMeshLibrary|CopyProceduralMeshfromStaticMeshComponent _array_element 0 _returnvalue true)
    (bind _vertices (Class|KismetProceduralMeshLibrary|GetSectionfromProceduralMesh _returnvalue))
    (Class|ProceduralMeshComponent|AddCollisionConvexMesh _returnvalue _vertices))
  (Actor|DestroyActor ActorSource))

(event Custom|Slice
  (params (Position :type Vector) (Normal :type Vector))
  (for _array_element (Actor|GetComponentsByClass "/Script/ProceduralMeshComponent.ProceduralMeshComponent")
    (Class|KismetProceduralMeshLibrary|SliceProceduralMesh _array_element Position Normal false "NoCap")))

(fn ConstructionScript)